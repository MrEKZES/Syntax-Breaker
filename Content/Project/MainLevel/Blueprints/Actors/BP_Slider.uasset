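; Clickable five-position slider that aims the satellite plate and drives the lost-signal event in the main level.
; Each click cycles the position, moves the switcher, rotates the plate and updates the monitor's answer array.
; A looping timer periodically re-randomizes the target once matched.
; A mismatch shows the LostSignal HUD and flashes the target on the monitor; matching clears it and requests a new question.
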(event OnClicked(Cube)
  (params (TouchedComponent :type Primitive%20Component%20Object%20Reference) (ButtonPressed :type Key%20Structure :default "None"))
  (bind _bp_monitor (Variables|Default|GetBP_Monitor))
  (bind _trueposition (Variables|Default|GetTruePosition))
  (bind _bp_monitor_2 (Variables|Default|GetBP_Monitor))
  (bind _bp_monitor_3 (Variables|Default|GetBP_Monitor))
  (bind _switcher (Variables|Default|GetSwitcher))
  (bind _arrays (Variables|/Game/Project/MainLevel/Blueprints/Actors/BP_Monitor.BP_Monitor_C|GetArrays _bp_monitor))
  (bind _as_bp_hudmain_level (Variables|/Game/Project/MainLevel/Blueprints/Actors/BP_Monitor.BP_Monitor_C|GetAs%20BP%20HUDMain%20Level _bp_monitor_2))
  (bind _as_wbp_monitor (Variables|/Game/Project/MainLevel/Blueprints/Actors/BP_Monitor.BP_Monitor_C|GetAs%20WBP%20Monitor _bp_monitor_3))
  (bind _as_bp_hudmain_level_2 (Variables|/Game/Project/MainLevel/Blueprints/Actors/BP_Monitor.BP_Monitor_C|GetAs%20BP%20HUDMain%20Level _bp_monitor_3))
  (bind _lostsignal (Variables|/Game/Project/MainLevel/Blueprints/UI/BP_HUDMainLevel.BP_HUDMainLevel_C|GetLostSignal _as_bp_hudmain_level))
  (bind _lostsignal_2 (Variables|/Game/Project/MainLevel/Blueprints/UI/BP_HUDMainLevel.BP_HUDMainLevel_C|GetLostSignal _as_bp_hudmain_level_2))
  (if (< (Variables|Default|GetPosition) 5)
    (Math|Integer|IncrementInt (Variables|Default|GetPosition)
      (:%20%20
        _))
    (else
      (Variables|Default|SetPosition 1)))
  (Development|PrintString (Utilities|String|ToString(Integer) (Variables|Default|GetPosition)))
  (Utilities|Array|SetArrayElem _arrays 6 (Utilities|Struct|MakeS_ArraysOfID (.question (Utilities|Array|Get(acopy) _arrays 6)) (Utilities|Array|MakeArray (Variables|Default|GetPosition))))
  (Default|SetRotaitonPlate (Variables|Default|GetSatelite%20plate) (Variables|Default|GetPosition))
  (Utilities|FlowControl|Sequence
    (:then_0
      (switch int (Variables|Default|GetPosition)
        (:1
          (Transformation|SetRelativeLocation _switcher "15.603820,0.000000,5.403940" false false))
        (:2
          (Transformation|SetRelativeLocation _switcher "7.801910,0.000000,5.403940" false false))
        (:3
          (Transformation|SetRelativeLocation _switcher "0.000000,0.000000,5.403940" false false))
        (:4
          (Transformation|SetRelativeLocation _switcher "-7.801910,0.000000,5.403940" false false))
        (:5
          (Transformation|SetRelativeLocation _switcher "-15.603821,0.000000,5.403940" false false))))
    (:then_1
      (if (== (Variables|Default|GetTruePosition) (Variables|Default|GetPosition))
        (if (UserInterface|Viewport|IsinViewport _lostsignal)
          (Widget|RemovefromParent _lostsignal)
          (Utilities|Time|PauseTimerbyHandle (Variables|Default|GetTimer))
          (Utilities|FlowControl|Delay 1.0)
          (Default|NewQuestion _bp_monitor_2))
        (else
          (if (UserInterface|Viewport|IsinViewport _lostsignal_2)
            (Widget|RemovefromParent _lostsignal_2))
          (Default|AddLostSignal _as_bp_hudmain_level_2 (Utilities|Text|ToText(Integer) (Variables|Default|GetTruePosition)))
          (bind _returnvalue (Utilities|Time|SetTimerbyEvent (delegate Custom|SetShifrInLostSignal) 1.0 true))
          (Variables|Default|SetTimer _returnvalue)
          (Default|UpdateShifrImages _as_wbp_monitor (Utilities|Array|MakeArray 23 _trueposition 23 _trueposition 23 _trueposition 23 _trueposition 23 _trueposition))
          (Utilities|FlowControl|Delay 0.5)
          (Default|UpdateShifrImages _as_wbp_monitor))))))

(event Custom|SetTruePosition
  (bind _bp_monitor (Variables|Default|GetBP_Monitor))
  (bind _as_wbp_monitor (Variables|/Game/Project/MainLevel/Blueprints/Actors/BP_Monitor.BP_Monitor_C|GetAs%20WBP%20Monitor _bp_monitor))
  (bind _as_bp_hudmain_level (Variables|/Game/Project/MainLevel/Blueprints/Actors/BP_Monitor.BP_Monitor_C|GetAs%20BP%20HUDMain%20Level _bp_monitor))
  (bind _lostsignal (Variables|/Game/Project/MainLevel/Blueprints/UI/BP_HUDMainLevel.BP_HUDMainLevel_C|GetLostSignal _as_bp_hudmain_level))
  (if (== (Variables|Default|GetPosition) (Variables|Default|GetTruePosition))
    (Variables|Default|SetTruePosition (Math|Random|RandomIntegerinRange 1 5))
    (if (!= (Variables|Default|GetPosition) (Variables|Default|GetTruePosition))
      (Development|PrintString "Hello")
      (Default|NewQuestion _bp_monitor)
      (if (UserInterface|Viewport|IsinViewport _lostsignal)
        (Widget|RemovefromParent _lostsignal))
      (Default|AddLostSignal _as_bp_hudmain_level (Utilities|Text|ToText(Integer) (Variables|Default|GetTruePosition)))
      (bind _returnvalue (Utilities|Time|SetTimerbyEvent (delegate Custom|SetShifrInLostSignal) 1.0 true))
      (Variables|Default|SetTimer _returnvalue)
      (Default|UpdateShifrImages _as_wbp_monitor (Utilities|Array|MakeArray 23 (Variables|Default|GetTruePosition) 23 (Variables|Default|GetTruePosition) 23 (Variables|Default|GetTruePosition) 23 (Variables|Default|GetTruePosition) 23 (Variables|Default|GetTruePosition)))
      (Utilities|FlowControl|Delay 0.5)
      (Default|UpdateShifrImages _as_wbp_monitor))))

(event Custom|SetShifrInLostSignal
  (bind _trueposition (Variables|Default|GetTruePosition))
  (bind _bp_monitor (Variables|Default|GetBP_Monitor))
  (bind _as_wbp_monitor (Variables|/Game/Project/MainLevel/Blueprints/Actors/BP_Monitor.BP_Monitor_C|GetAs%20WBP%20Monitor _bp_monitor))
  (Default|UpdateShifrImages _as_wbp_monitor (Utilities|Array|MakeArray 23 _trueposition 23 _trueposition 23 _trueposition 23 _trueposition 23 _trueposition))
  (Utilities|FlowControl|Delay 0.5)
  (Default|UpdateShifrImages _as_wbp_monitor))

(event EventBeginPlay
  (bind _trueposition (Variables|Default|GetTruePosition))
  (bind _switcher (Variables|Default|GetSwitcher))
  (Utilities|FlowControl|Delay 0.0)
  (bind _returnvalue (Actor|GetActorOfClass "/Game/Project/MainLevel/Blueprints/Actors/BP_Monitor.BP_Monitor_C"))
  (Variables|Default|SetBP_Monitor _returnvalue)
  (bind _returnvalue_2 (Actor|GetActorOfClass "/Game/Project/MainLevel/Blueprints/Actors/BP_SatellitePlate.BP_SatellitePlate_C"))
  (Variables|Default|SetSatelite%20plate _returnvalue_2)
  (Utilities|Time|SetTimerbyEvent (delegate Custom|SetTruePosition) 55.0 true)
  (Development|PrintString (Utilities|String|ToString(Integer) (Variables|Default|GetPosition)))
  (Utilities|Array|SetArrayElem (Variables|/Game/Project/MainLevel/Blueprints/Actors/BP_Monitor.BP_Monitor_C|GetArrays (Variables|Default|GetBP_Monitor)) 6 (Utilities|Struct|MakeS_ArraysOfID (.question (Utilities|Array|Get(acopy) (Variables|/Game/Project/MainLevel/Blueprints/Actors/BP_Monitor.BP_Monitor_C|GetArrays (Variables|Default|GetBP_Monitor)) 6)) (Utilities|Array|MakeArray (Variables|Default|GetPosition))))
  (Default|SetRotaitonPlate (Variables|Default|GetSatelite%20plate) (Variables|Default|GetPosition))
  (Utilities|FlowControl|Sequence
    (:then_0
      (switch int (Variables|Default|GetPosition)
        (:1
          (Transformation|SetRelativeLocation _switcher "15.603820,0.000000,5.403940" false false))
        (:2
          (Transformation|SetRelativeLocation _switcher "7.801910,0.000000,5.403940" false false))
        (:3
          (Transformation|SetRelativeLocation _switcher "0.000000,0.000000,5.403940" false false))
        (:4
          (Transformation|SetRelativeLocation _switcher "-7.801910,0.000000,5.403940" false false))
        (:5
          (Transformation|SetRelativeLocation _switcher "-15.603821,0.000000,5.403940" false false))))
    (:then_1
      (if (== (Variables|Default|GetTruePosition) (Variables|Default|GetPosition))
        (if (UserInterface|Viewport|IsinViewport (Variables|/Game/Project/MainLevel/Blueprints/UI/BP_HUDMainLevel.BP_HUDMainLevel_C|GetLostSignal (Variables|/Game/Project/MainLevel/Blueprints/Actors/BP_Monitor.BP_Monitor_C|GetAs%20BP%20HUDMain%20Level (Variables|Default|GetBP_Monitor))))
          (Widget|RemovefromParent (Variables|/Game/Project/MainLevel/Blueprints/UI/BP_HUDMainLevel.BP_HUDMainLevel_C|GetLostSignal (Variables|/Game/Project/MainLevel/Blueprints/Actors/BP_Monitor.BP_Monitor_C|GetAs%20BP%20HUDMain%20Level (Variables|Default|GetBP_Monitor))))
          (Utilities|Time|PauseTimerbyHandle (Variables|Default|GetTimer))
          (Utilities|FlowControl|Delay 1.0)
          (Default|NewQuestion (Variables|Default|GetBP_Monitor)))
        (else
          (if (UserInterface|Viewport|IsinViewport (Variables|/Game/Project/MainLevel/Blueprints/UI/BP_HUDMainLevel.BP_HUDMainLevel_C|GetLostSignal (Variables|/Game/Project/MainLevel/Blueprints/Actors/BP_Monitor.BP_Monitor_C|GetAs%20BP%20HUDMain%20Level (Variables|Default|GetBP_Monitor))))
            (Widget|RemovefromParent (Variables|/Game/Project/MainLevel/Blueprints/UI/BP_HUDMainLevel.BP_HUDMainLevel_C|GetLostSignal (Variables|/Game/Project/MainLevel/Blueprints/Actors/BP_Monitor.BP_Monitor_C|GetAs%20BP%20HUDMain%20Level (Variables|Default|GetBP_Monitor)))))
          (Default|AddLostSignal (Variables|/Game/Project/MainLevel/Blueprints/Actors/BP_Monitor.BP_Monitor_C|GetAs%20BP%20HUDMain%20Level (Variables|Default|GetBP_Monitor)) (Utilities|Text|ToText(Integer) (Variables|Default|GetTruePosition)))
          (bind _returnvalue_3 (Utilities|Time|SetTimerbyEvent (delegate Custom|SetShifrInLostSignal) 1.0 true))
          (Variables|Default|SetTimer _returnvalue_3)
          (Default|UpdateShifrImages (Variables|/Game/Project/MainLevel/Blueprints/Actors/BP_Monitor.BP_Monitor_C|GetAs%20WBP%20Monitor (Variables|Default|GetBP_Monitor)) (Utilities|Array|MakeArray 23 _trueposition 23 _trueposition 23 _trueposition 23 _trueposition 23 _trueposition))
          (Utilities|FlowControl|Delay 0.5)
          (Default|UpdateShifrImages (Variables|/Game/Project/MainLevel/Blueprints/Actors/BP_Monitor.BP_Monitor_C|GetAs%20WBP%20Monitor (Variables|Default|GetBP_Monitor))))))))

(fn ConstructionScript)