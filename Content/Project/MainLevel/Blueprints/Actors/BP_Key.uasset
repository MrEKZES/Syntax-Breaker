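; BP_Key is a clickable key actor that types its symbol into a BP_Monitor.
; On BeginPlay it finds the monitor in the level and enables click events on the player controller.
; Clicking its cube plays the key's press animation and adds its KeyID to the monitor's answer.
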(event OnClicked(CLICK)
  (params (TouchedComponent :type Primitive%20Component%20Object%20Reference) (ButtonPressed :type Key%20Structure :default "None")))

(event OnClicked(Cube)
  (params (TouchedComponent :type Primitive%20Component%20Object%20Reference) (ButtonPressed :type Key%20Structure :default "None"))
  ;[0.15 0.15 0.15 0.5] Type symbol
  (Components|Animation|PlayAnimation (Variables|Default|GetCLICK) "/Game/Project/MainLevel/Meshes/Keyboard/Key/CLICK_Anim_Armature_ArmatureAction.CLICK_Anim_Armature_ArmatureAction" false)
  (CallFunction|KeyInput))

(event Custom|Key%20Input
  ;[0.15 0.15 0.15 0.5] Type symbol
  (Default|AddNewIDinAnswer (Variables|Default|GetBP_Monitor) (Variables|Default|GetKeyID)))

(event EventBeginPlay
  ;[0.15 0.15 0.15 0.5] Cast to BP_Monitor
  (bind _returnvalue (Actor|GetActorOfClass "/Game/Project/MainLevel/Blueprints/Actors/BP_Monitor.BP_Monitor_C"))
  (Variables|Default|SetBP_Monitor _returnvalue)
  ;[0.15 0.15 0.15 0.5] Enable Click Events
  (Variables|/Script/Engine.PlayerController|SetbEnableClickEvents (Game|GetPlayerController 0) true))

(fn ConstructionScript)