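; BP_Monitor is an in-world monitor actor that runs a cipher puzzle, showing a random question and collecting an answer as a list of IDs.
; It links itself to its WBP_Monitor widget, which displays the question and the current input.
; Events append IDs up to a ten-entry cap or remove the last.
; The answer check is a print-only stub with apparently inverted branches: a match prints "-HP", a mismatch loads a new question.
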(event Custom|AswerIsRight
  (if (Utilities|Array|Identical (Variables|Default|GetInputIDArray) (.trueanswer (Utilities|Array|Get(acopy) (Variables|Default|GetArrays) (Variables|Default|GetIDOfQuestion))))
    ;[0.15 0.15 0.15 0.5] -HP Player (Damage)
    (Development|PrintString "-HP" true true "(R=1.000000,G=0.000000,B=0.000000,A=1.000000)" 1e+01)
    (else
      (Development|PrintString "TrueAnswer" true true "(R=0.000000,G=1.000000,B=0.000000,A=1.000000)" 1e+01)
      (CallFunction|NewQuestion))))

(event Custom|NewQuestion
  (bind _arrays (Variables|Default|GetArrays))
  (bind _output_get (Variables|Default|SetIDOfQuestion (Math|Random|RandomIntegerinRange 0 (Utilities|Array|LastIndex _arrays))))
  (Default|UpdateShifrImages (Variables|Default|GetAs%20WBP%20Monitor) (.question (Utilities|Array|Get(acopy) _arrays _output_get))))

(event Custom|AddNewIDInAnswer
  (params (NewID :type Integer%20%28by%20ref%29))
  (bind _inputidarray (Variables|Default|GetInputIDArray))
  ;[0.15 0.15 0.15 0.5] Answer Editable Event
  (if (< (Utilities|Array|LastIndex _inputidarray) 9)
    (Utilities|Array|Add _inputidarray NewID)
    (Default|UpdateInputImages (Variables|Default|GetAs%20WBP%20Monitor) (Variables|Default|GetInputIDArray))))

(event Custom|RemoveLastID
  (bind _inputidarray (Variables|Default|GetInputIDArray))
  ;[0.15 0.15 0.15 0.5] Answer Editable Event
  (Utilities|Array|RemoveIndex _inputidarray (Utilities|Array|LastIndex _inputidarray))
  (Default|UpdateInputImages (Variables|Default|GetAs%20WBP%20Monitor) (Variables|Default|GetInputIDArray)))

(event EventBeginPlay
  (bind _aswbp_monitor (Utilities|Casting|CastToWBP_Monitor (UserInterface|GetWidget (Variables|Default|GetWBP_Monitor))))
  (bind _output_get (Variables|Default|SetAs%20WBP%20Monitor _aswbp_monitor))
  (Variables|/Game/Project/MainLevel/Blueprints/UI/Widgets/WBP_Monitor.WBP_Monitor_C|SetBP_Monitor _output_get self)
  (Utilities|FlowControl|Delay 0.002)
  (CallFunction|NewQuestion))

(fn ConstructionScript)