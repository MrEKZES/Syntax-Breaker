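; BP_Thermometer is an actor showing a drifting temperature that feeds an answer on BP_Monitor.
; A looping timer nudges the value by a small random integer, using a range check to steer it within bounds.
; In-range updates write the tens and units digits as the true answer for the monitor's first question and rescale the Cylinder's height to match.
; Each random node use re-rolls, so checked and applied steps can differ.
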(event Custom|SetNewTempeture
  (bind _returnvalue (Math|Random|RandomIntegerinRange -1 1))
  (bind _cylinder (Variables|Default|GetCylinder))
  (bind _monitor (Variables|Default|GetMonitor))
  (bind _returnvalue_2 (Transformation|GetWorldScale _cylinder))
  (bind _arrays (Variables|/Game/Project/MainLevel/Blueprints/Actors/BP_Monitor.BP_Monitor_C|GetArrays _monitor))
  (if (and (< (+ (Variables|Default|GetTempeture) _returnvalue) 90) (> (+ (Variables|Default|GetTempeture) _returnvalue) 15))
    (Variables|Default|SetTempeture (+ (Variables|Default|GetTempeture) _returnvalue))
    ;[0.15 0.15 0.15 0.5] Set true answer
    (Utilities|Array|SetArrayElem _arrays 0 (Utilities|Struct|MakeS_ArraysOfID (.question (Utilities|Array|Get(acopy) _arrays)) (Utilities|Array|MakeArray (/ (Variables|Default|GetTempeture) 10) (Math|Integer|%(Integer) (Variables|Default|GetTempeture) 10))))
    ;[0.15 0.15 0.15 0.5] Set Scale
    (Transformation|SetRelativeScale3D _cylinder (Math|Vector|MakeVector (.x _returnvalue_2) (.y _returnvalue_2) (/ (Variables|Default|GetTempeture) 10)))
    (else
      (Variables|Default|SetTempeture (- (Variables|Default|GetTempeture) _returnvalue)))))

(event EventBeginPlay
  (bind _cylinder (Variables|Default|GetCylinder))
  (bind _returnvalue (Transformation|GetWorldScale _cylinder))
  (bind _returnvalue_2 (Actor|GetActorOfClass "/Game/Project/MainLevel/Blueprints/Actors/BP_Monitor.BP_Monitor_C"))
  (Variables|Default|SetMonitor _returnvalue_2)
  (Utilities|Time|SetTimerbyEvent (delegate Custom|SetNewTempeture) 3e+01 true)
  ;[0.15 0.15 0.15 0.5] Starter Scale
  (Transformation|SetRelativeScale3D _cylinder (Math|Vector|MakeVector (.x _returnvalue) (.y _returnvalue) (/ (Variables|Default|GetTempeture) 10))))

(fn ConstructionScript)