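; Main-level player camera actor that becomes the view target and doubles as the player's state holder.
; Each tick it offsets from its start position by normalized cursor position, adds axis input to pitch and yaw, and prints debug stats.
; Keys handle clamped FOV zoom, the HUD pause menu and a debug monitor question.
; Events control cigarette visibility and smoke, and decrement health, opening the main menu once depleted.
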(event Custom|Get%20Cigarette
  ;[0.15 0.15 0.15 0.5] Cigarette mechanics
  (bind _output_get (Variables|CigfareteVars|SetCigaretteVisibility true))
  (Rendering|SetVisibility (Variables|Default|GetCigarette) _output_get false))

(event Custom|Light%20a%20cigarette
  ;[0.15 0.15 0.15 0.5] Cigarette mechanics
  (if (Variables|CigfareteVars|GetCigaretteVisibility)
    (if (not (Variables|/Script/Engine.SceneComponent|GetbVisible (Variables|Default|GetP_Smoke_A)))
      (Audio|PlaySound2D "/Game/Project/MainLevel/Sounds/CigaretteCracking.CigaretteCracking" 1.0 1.0 0.0 0 0)
      (Utilities|FlowControl|Delay 1.8)
      (Rendering|SetVisibility (Variables|Default|GetP_Smoke_A) true false))))

(event Custom|TakeDamage
  ;[0.15 0.15 0.15 0.5] Take damage
  (if (>= (Variables|Default|GetHealth) 1)
    (Variables|Default|SetHealth (- (Variables|Default|GetHealth) 1))
    (else
      (Utilities|FlowControl|Delay 1.0)
      (Game|OpenLevel(byName) "Lvl_MainMenu"))))

(event Custom|Put%20out%20the%20cigarette
  ;[0.15 0.15 0.15 0.5] Cigarette mechanics
  (if (Variables|CigfareteVars|GetCigaretteVisibility)
    (bind _output_get (Variables|CigfareteVars|SetCigaretteVisibility false))
    (Rendering|SetVisibility (Variables|Default|GetCigarette) _output_get false)
    (if (Variables|/Script/Engine.SceneComponent|GetbVisible (Variables|Default|GetP_Smoke_A))
      (Rendering|SetVisibility (Variables|Default|GetP_Smoke_A) false false))))

(event EventBeginPlay
  (bind _returnvalue (Game|GetPlayerController 0))
  (Variables|/Script/Engine.PlayerController|SetbShowMouseCursor _returnvalue true)
  (Input|SetInputModeGameOnly _returnvalue false)
  (Game|Player|SetViewTargetwithBlend _returnvalue self 0.0 "VTBlend_Linear" 0.0 false)
  (Variables|CameraStats|SetStartPosition (Transformation|GetActorLocation))
  (bind _returnvalue_2 (Actor|GetActorOfClass "/Game/Project/MainLevel/Blueprints/Actors/BP_Key.BP_Key_C"))
  (Variables|Links|SetBP_Keyboard _returnvalue_2)
  (bind _asbp_hudmain_level (Utilities|Casting|CastToBP_HUDMainLevel (HUD|GetHUD (Game|GetPlayerController 0))))
  (Variables|Links|SetAs%20BP%20HUDMain%20Level _asbp_hudmain_level)
  (bind _returnvalue_3 (Actor|GetActorOfClass "/Game/Project/MainLevel/Blueprints/Actors/BP_Monitor.BP_Monitor_C"))
  (Variables|Links|SetBP_Monitor _returnvalue_3))

(event EventTick
  (params (DeltaSeconds :type Float%20%28single-precision%29))
  (bind _returnvalue (Game|GetPlayerController 0))
  (bind _camera (Variables|Default|GetCamera))
  (bind _speed (Variables|CameraStats|GetSpeed))
  (bind (_locationx _locationy) (Game|Player|GetMousePosition _returnvalue))
  (bind (_sizex _sizey) (HUD|GetViewportSize _returnvalue))
  (bind _returnvalue_2 (Transformation|GetWorldRotation _camera))
  (bind (_roll _pitch _yaw) (Math|Rotator|BreakRotator _returnvalue_2))
  (bind _returnvalue_3 (Math|Conversions|ToFloat(Integer) _sizey))
  (bind _returnvalue_4 (Math|Conversions|ToFloat(Integer) _sizex))
  (bind _returnvalue_5 (/ _returnvalue_3 2.0))
  (bind _returnvalue_6 (/ _returnvalue_4 2.0))
  ;[0.15 0.15 0.15 0.5] Camera Settings
  (Transformation|SetActorLocationAndRotation (+ (* (* (/ (- _locationx _returnvalue_6) _returnvalue_6) (* 1.0 _speed)) (Math|Vector|GetRightVector _returnvalue_2)) (Variables|CameraStats|GetStartPosition) (* (* (* _speed -1.0) (/ (- _locationy _returnvalue_5) _returnvalue_5)) (Math|Vector|GetUpVector _returnvalue_2))) (Math|Rotator|MakeRotator _roll (+ _pitch (/ (Class|Actor|GetInputAxisKeyValue) (Variables|CameraStats|GetMouseSpeedDevider))) (+ _yaw (/ (Class|Actor|GetInputAxisKeyValue) (Variables|CameraStats|GetMouseSpeedDevider)))))
  ;[0.15 0.15 0.15 0.5] Camera stats in string
  (Development|PrintString (Utilities|String|ToString(Transform) (Transformation|GetActorTransform)) true true "(R=0.000000,G=0.660000,B=1.000000,A=1.000000)" 0.0)
  ;[0.15 0.15 0.15 0.5] Cur FOV in string
  (Development|PrintString (Utilities|String|ToString(Float) (Variables|/Script/Engine.CameraComponent|GetFieldOfView (Variables|Default|GetCamera))) true true "(R=0.000000,G=0.660000,B=1.000000,A=1.000000)" 0.0))

(event Input|MouseEvents|MouseWheelUp
  (params (Key :type Key%20Structure :default "None"))
  (bind _camera (Variables|Default|GetCamera))
  (bind _camera_2 (Variables|Default|GetCamera))
  ;[0.15 0.15 0.15 0.5] Camera zoom
  (:Pressed
    (Camera|SetFieldOfView _camera_2 (- (Variables|/Script/Engine.CameraComponent|GetFieldOfView _camera_2) (Variables|CameraStats|GetFieldOfViewAdder)))
    (if (<= (Variables|/Script/Engine.CameraComponent|GetFieldOfView _camera) 2e+01)
      (Camera|SetFieldOfView _camera 2e+01))))

(event Input|MouseEvents|LeftMouseButton
  (params (Key :type Key%20Structure :default "None"))
  ;[0.15 0.15 0.15 0.5] Camera Settings
  (:Released
    (Input|SetInputModeGameOnly (Game|GetPlayerController 0) false)))

(event Input|KeyboardEvents|Q
  (params (Key :type Key%20Structure :default "None")))

(event Input|KeyboardEvents|E
  (params (Key :type Key%20Structure :default "None")))

(event Input|KeyboardEvents|9
  (params (Key :type Key%20Structure :default "None"))
  ;[1 0 0] DEBUGING (DELETE THIS)
  (:Pressed
    (Default|NewQuestion (Variables|Links|GetBP_Monitor))))

(event Input|MouseEvents|MouseWheelDown
  (params (Key :type Key%20Structure :default "None"))
  (bind _camera (Variables|Default|GetCamera))
  (bind _camera_2 (Variables|Default|GetCamera))
  ;[0.15 0.15 0.15 0.5] Camera zoom
  (:Pressed
    (Camera|SetFieldOfView _camera (+ (Variables|/Script/Engine.CameraComponent|GetFieldOfView _camera) (Variables|CameraStats|GetFieldOfViewAdder)))
    (if (>= (Variables|/Script/Engine.CameraComponent|GetFieldOfView _camera_2) 1.3e+02)
      (Camera|SetFieldOfView _camera_2 1.3e+02))))

(event Input|MouseEvents|MiddleMouseButton
  (params (Key :type Key%20Structure :default "None"))
  ;[0.15 0.15 0.15 0.5] Camera Settings
  (:Released
    (Input|SetInputModeGameOnly (Game|GetPlayerController 0) false)))

(event Input|MouseEvents|RightMouseButton
  (params (Key :type Key%20Structure :default "None"))
  ;[0.15 0.15 0.15 0.5] Camera Settings
  (:Released
    (Input|SetInputModeGameOnly (Game|GetPlayerController 0) false)))

(event Input|MouseEvents|ThumbMouseButton
  (params (Key :type Key%20Structure :default "None"))
  ;[0.15 0.15 0.15 0.5] Camera Settings
  (:Released
    (Input|SetInputModeGameOnly (Game|GetPlayerController 0) false)))

(event Input|MouseEvents|ThumbMouseButton2
  (params (Key :type Key%20Structure :default "None"))
  ;[0.15 0.15 0.15 0.5] Camera Settings
  (:Released
    (Input|SetInputModeGameOnly (Game|GetPlayerController 0) false)))

(event Input|KeyboardEvents|P
  (params (Key :type Key%20Structure :default "None"))
  ;[0.15 0.15 0.15 0.5] Pause menu
  (:Pressed
    (Default|AddPauseMenu (Variables|Links|GetAs%20BP%20HUDMain%20Level))))

(fn ConstructionScript)