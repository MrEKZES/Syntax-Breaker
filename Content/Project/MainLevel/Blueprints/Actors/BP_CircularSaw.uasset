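; Circular saw actor that plays a staged kill sequence on an animated disc mesh, exposed as three events with no trigger logic of its own.
; The start event slides the disc out along its relative Y with a timeline, and the spike event plays a one-shot spike-opening animation.
; The death event loops the spin animation while a Launch timeline moves the disc, with a saw sound and delayed screams.
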(event Custom|PlayAnimaitionSpiek
  (Components|Animation|PlayAnimation (Variables|Default|Getdisc_anim_uv) "/Game/Project/MainLevel/Meshes/Disk/disc_anim_uv_Anim_Armature_Spikes.disc_anim_uv_Anim_Armature_Spikes" false)
  (Audio|PlaySound2D "/Game/Project/MainLevel/Sounds/OpenSpikes.OpenSpikes" 1.0 1.0 0.0 0 0))

(event Custom|PlayAnimaitionDeath
  (Components|Animation|PlayAnimation (Variables|Default|Getdisc_anim_uv) "/Game/Project/MainLevel/Meshes/Disk/disc_anim_uv_Anim_Armature_Spin.disc_anim_uv_Anim_Armature_Spin" true)
  (Utilities|FlowControl|Sequence
    (:then_0
      (bind _y (Timeline|Launch Play)
        (:Update
          (Transformation|SetRelativeLocation (Variables|Default|Getdisc_anim_uv) (Math|Vector|MakeVector 0.0 _y 0.0) false false))))
    (:then_1
      (Audio|PlaySound2D "/Game/Project/MainLevel/Sounds/RollSaw.RollSaw" 1.0 1.0 0.0 0 0)
      (Utilities|FlowControl|Delay 1.8)
      (Audio|PlaySound2D "/Game/Project/MainLevel/Sounds/Screams.Screams" 1.0 1.0 0.0 0 0))))

(event Custom|PlayAnimaitonStart
  (Audio|PlaySound2D "/Game/Project/MainLevel/Sounds/DiskOut.DiskOut" 1.0 1.0 0.0 0 0)
  (bind _y (Timeline|Timeline Play)
    (:Update
      (Transformation|SetRelativeLocation (Variables|Default|Getdisc_anim_uv) (Math|Vector|MakeVector 0.0 _y 0.0) false false))))

(fn ConstructionScript)