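; Radio actor with a screen widget whose slowly drifting frequency serves as the answer to one of BP_Monitor's questions.
; On BeginPlay it caches the widget and monitor, then starts a looping timer that randomly nudges the whole and decimal parts within loose bounds.
; At start and after each drift, it writes the frequency's digits into the monitor's question array as the true answer, keeping the question text.
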(event Custom|SetRadioWave
  (bind _returnvalue (Math|Random|RandomIntegerinRange -1 1))
  (bind _returnvalue_2 (Math|Random|RandomIntegerinRange -1 1))
  (bind _monitor (Variables|Default|GetMonitor))
  (bind _arrays (Variables|/Game/Project/MainLevel/Blueprints/Actors/BP_Monitor.BP_Monitor_C|GetArrays _monitor))
  (if (and (< (+ (Variables|Default|GetWave) _returnvalue_2) 90) (> (+ (Variables|Default|GetWave) _returnvalue_2) 30))
    (Variables|Default|SetWave (+ (Variables|Default|GetWave) _returnvalue_2))
    (else
      (Variables|Default|SetWave (- (Variables|Default|GetWave) _returnvalue_2))))
  (if (and (< (+ (Variables|Default|GetWaveSecond) _returnvalue) 9) (> (+ (Variables|Default|GetWaveSecond) _returnvalue) 1))
    (Variables|Default|SetWaveSecond (+ (Variables|Default|GetWaveSecond) _returnvalue))
    (else
      (Variables|Default|SetWaveSecond (- (Variables|Default|GetWaveSecond) _returnvalue))))
  ;[0.15 0.15 0.15 0.5] Set true answer
  (Utilities|Array|SetArrayElem _arrays 4 (Utilities|Struct|MakeS_ArraysOfID (.question (Utilities|Array|Get(acopy) _arrays 4)) (Utilities|Array|MakeArray (/ (Variables|Default|GetWave) 10) (Math|Integer|%(Integer) (Variables|Default|GetWave) 10) 11 (Variables|Default|GetWaveSecond)))))

(event EventBeginPlay
  (bind _wave (Variables|Default|GetWave))
  (bind _aswbp_radio (Utilities|Casting|CastToWBP_Radio (UserInterface|GetWidget (Variables|Default|GetWidget))))
  (Variables|Default|SetAs%20WBP%20Radio _aswbp_radio)
  (bind _returnvalue (Actor|GetActorOfClass "/Game/Project/MainLevel/Blueprints/Actors/BP_Monitor.BP_Monitor_C"))
  (Variables|Default|SetMonitor _returnvalue)
  (Utilities|Time|SetTimerbyEvent (delegate Custom|SetRadioWave) 2e+01 true)
  ;[0.15 0.15 0.15 0.5] Set true answer
  (Utilities|Array|SetArrayElem (Variables|/Game/Project/MainLevel/Blueprints/Actors/BP_Monitor.BP_Monitor_C|GetArrays (Variables|Default|GetMonitor)) 4 (Utilities|Struct|MakeS_ArraysOfID (.question (Utilities|Array|Get(acopy) (Variables|/Game/Project/MainLevel/Blueprints/Actors/BP_Monitor.BP_Monitor_C|GetArrays (Variables|Default|GetMonitor)) 4)) (Utilities|Array|MakeArray (/ _wave 10) (Math|Integer|%(Integer) _wave 10) 11 (Variables|Default|GetWaveSecond)))))

(fn ConstructionScript)