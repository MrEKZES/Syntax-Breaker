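; BP_Guide is a clickable actor in the main level that toggles the tutorial display.
; On BeginPlay it enables click events on the player controller and caches references to BP_MainCamera and BP_HUDMainLevel, though the camera reference is unused in this graph.
; Clicks on its Guide component drive a FlipFlop that alternates between calling AddTutorial on the HUD and removing the HUD's tutorial widget from its parent.
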(event OnClicked(Guide)
  (params (TouchedComponent :type Primitive%20Component%20Object%20Reference) (ButtonPressed :type Key%20Structure))
  (Utilities|FlowControl|FlipFlop
    (:A
      (Default|AddTutorial (Variables|Default|GetBP%20HUD%20MainLevel)))
    (:B
      (Widget|RemovefromParent (Variables|/Game/Project/MainLevel/Blueprints/UI/BP_HUDMainLevel.BP_HUDMainLevel_C|GetWBP_Tutorial (Variables|Default|GetBP%20HUD%20MainLevel))))))

(event EventBeginPlay
  (bind _returnvalue (Actor|GetActorOfClass "/Game/Project/MainLevel/Blueprints/Actors/BP_MainCamera.BP_MainCamera_C"))
  (Variables|Default|SetBP%20Main%20Canera _returnvalue)
  ;[0.15 0.15 0.15 0.5] Enable Click Events
  (Variables|/Script/Engine.PlayerController|SetbEnableClickEvents (Game|GetPlayerController 0) true)
  (bind _returnvalue_2 (Actor|GetActorOfClass "/Game/Project/MainLevel/Blueprints/UI/BP_HUDMainLevel.BP_HUDMainLevel_C"))
  (Variables|Default|SetBP%20HUD%20MainLevel _returnvalue_2))

(fn ConstructionScript)