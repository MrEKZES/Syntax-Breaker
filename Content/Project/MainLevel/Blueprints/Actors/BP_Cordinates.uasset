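; Coordinates actor that keeps two drifting numbers and feeds them to BP_Monitor as a puzzle answer.
; BeginPlay caches its coordinates widget and the monitor, writes the answer, and starts a looping 30-second timer.
; Each tick randomly nudges both numbers, loosely bounded to two digits since each check rolls separately from the applied step.
; Their digits, split by a separator code, overwrite the true answer of one fixed monitor question.
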(event Custom|SetCordinates
  (bind _returnvalue (Math|Random|RandomIntegerinRange -1 1))
  (bind _returnvalue_2 (Math|Random|RandomIntegerinRange -1 1))
  (bind _monitor (Variables|Default|GetMonitor))
  (bind _arrays (Variables|/Game/Project/MainLevel/Blueprints/Actors/BP_Monitor.BP_Monitor_C|GetArrays _monitor))
  (if (and (< (+ (Variables|Default|GetCordinates1) _returnvalue_2) 99) (> (+ (Variables|Default|GetCordinates1) _returnvalue_2) 11))
    (Variables|Default|SetCordinates1 (+ (Variables|Default|GetCordinates1) _returnvalue_2))
    (else
      (Variables|Default|SetCordinates1 (- (Variables|Default|GetCordinates1) _returnvalue_2))))
  (if (and (< (+ (Variables|Default|GetCordinates2) _returnvalue) 99) (> (+ (Variables|Default|GetCordinates2) _returnvalue) 11))
    (Variables|Default|SetCordinates2 (+ (Variables|Default|GetCordinates2) _returnvalue))
    (else
      (Variables|Default|SetCordinates2 (- (Variables|Default|GetCordinates2) _returnvalue))))
  ;[0.15 0.15 0.15 0.5] Set true answer
  (Utilities|Array|SetArrayElem _arrays 6 (Utilities|Struct|MakeS_ArraysOfID (.question (Utilities|Array|Get(acopy) _arrays 6)) (Utilities|Array|MakeArray (/ (Variables|Default|GetCordinates1) 10) (Math|Integer|%(Integer) (Variables|Default|GetCordinates1) 10) 11 (/ (Variables|Default|GetCordinates2) 10) (Math|Integer|%(Integer) (Variables|Default|GetCordinates2) 10)))))

(event EventBeginPlay
  (bind _cordinates1 (Variables|Default|GetCordinates1))
  (bind _cordinates2 (Variables|Default|GetCordinates2))
  (bind _aswbp_cordinates (Utilities|Casting|CastToWBP_Cordinates (UserInterface|GetWidget (Variables|Default|GetWidget))))
  (Variables|Default|SetAs%20WBP%20Cordinates _aswbp_cordinates)
  (bind _returnvalue (Actor|GetActorOfClass "/Game/Project/MainLevel/Blueprints/Actors/BP_Monitor.BP_Monitor_C"))
  (Variables|Default|SetMonitor _returnvalue)
  (Utilities|Time|SetTimerbyEvent (delegate Custom|SetCordinates) 3e+01 true)
  ;[0.15 0.15 0.15 0.5] Set true answer
  (Utilities|Array|SetArrayElem (Variables|/Game/Project/MainLevel/Blueprints/Actors/BP_Monitor.BP_Monitor_C|GetArrays (Variables|Default|GetMonitor)) 6 (Utilities|Struct|MakeS_ArraysOfID (.question (Utilities|Array|Get(acopy) (Variables|/Game/Project/MainLevel/Blueprints/Actors/BP_Monitor.BP_Monitor_C|GetArrays (Variables|Default|GetMonitor)) 6)) (Utilities|Array|MakeArray (/ _cordinates1 10) (Math|Integer|%(Integer) _cordinates1 10) 11 (/ _cordinates2 10) (Math|Integer|%(Integer) _cordinates2 10)))))

(fn ConstructionScript)