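; BP_BackSpace is a clickable 3D backspace key that deletes the last entry on the in-world BP_Monitor.
; On BeginPlay it finds the monitor in the level and enables mouse click events on the player controller.
; Clicking its cube alternates between two key sounds, plays the key press animation and calls RemoveLastID on the monitor.
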(event OnClicked(Cube)
  (params (TouchedComponent :type Primitive%20Component%20Object%20Reference) (ButtonPressed :type Key%20Structure))
  ;[0.15 0.15 0.15 0.5] Type symbol
  (Utilities|FlowControl|FlipFlop
    (:A
      (Audio|PlaySound2D "/Game/Project/MainLevel/Sounds/KeyPressed1.KeyPressed1" 1.0 1.0 0.0 0 0))
    (:B
      (Audio|PlaySound2D "/Game/Project/MainLevel/Sounds/KeyPressed2.KeyPressed2" 1.0 1.0 0.0 0 0)))
  (Components|Animation|PlayAnimation (Variables|Default|GetBACKSPACE) "/Game/Project/MainLevel/Meshes/Keyboard/BackSpace/BACKSPACE_Anim.BACKSPACE_Anim" false)
  (Default|RemoveLastID (Variables|Default|GetBP_Monitor)))

(event EventBeginPlay
  ;[0.15 0.15 0.15 0.5] Cast to BP_Monitor
  (bind _returnvalue (Actor|GetActorOfClass "/Game/Project/MainLevel/Blueprints/Actors/BP_Monitor.BP_Monitor_C"))
  (Variables|Default|SetBP_Monitor _returnvalue)
  ;[0.15 0.15 0.15 0.5] Enable Click Events
  (Variables|/Script/Engine.PlayerController|SetbEnableClickEvents (Game|GetPlayerController 0) true))

(fn ConstructionScript)